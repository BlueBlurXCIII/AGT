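; Player ball for a Rollerball game that tracks time, jump count and score, and creates the PlayerHUD widget on start.
; Tick-driven delays advance a stopwatch and steadily drain PPoints, while Space bar presses count jumps and cost points without applying movement here.
; Overlaps cast to four pickup tiers, each playing explosion effects and adding increasing rewards to a separate PPointsS total.
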(event EventActorBeginOverlap
  (params (OtherActor :type Actor%20Object%20Reference))
  (Utilities|FlowControl|Sequence
    (:then_0
      ;[1 1 1] Handle points (small)
      (bind _aspickup_c (Utilities|Casting|CastToPickup OtherActor))
      (Audio|PlaySoundatLocation "/Game/Audio/Explosion01.Explosion01" (Transformation|GetActorLocation))
      (Variables|Default|SetP_Points_S (+ (Variables|Default|GetP_Points_S) 100))
      (Effects|SpawnEmitteratLocation "/Game/Particles/P_Explosion.P_Explosion" (Transformation|GetActorLocation _aspickup_c)))
    (:then_1
      ;[1 1 1] Handle points (med)
      (bind _aspickupmed_c (Utilities|Casting|CastToPickupMed OtherActor))
      (Audio|PlaySoundatLocation "/Game/Audio/Explosion02.Explosion02" (Transformation|GetActorLocation))
      (Variables|Default|SetP_Points_S (+ (Variables|Default|GetP_Points_S) 300))
      (Effects|SpawnEmitteratLocation "/Game/Particles/P_Explosion.P_Explosion" (Transformation|GetActorLocation _aspickupmed_c)))
    (:then_2
      ;[1 1 1] Handle points (large)
      (bind _aspickuplarge_c (Utilities|Casting|CastToPickupLarge OtherActor))
      (Audio|PlaySoundatLocation "/Game/Audio/Explosion01.Explosion01" (Transformation|GetActorLocation))
      (Variables|Default|SetP_Points_S (+ (Variables|Default|GetP_Points_S) 1000))
      (Effects|SpawnEmitteratLocation "/Game/Particles/P_Explosion.P_Explosion" (Transformation|GetActorLocation _aspickuplarge_c)))
    (:then_3
      ;[1 1 1] Handle points (mega)
      (bind _asmegasphere_c (Utilities|Casting|CastToMegaSphere OtherActor))
      (Audio|PlaySoundatLocation "/Game/Audio/Explosion01.Explosion01" (Transformation|GetActorLocation))
      (Variables|Default|SetP_Points_S (+ (Variables|Default|GetP_Points_S) 10000))
      (Effects|SpawnEmitteratLocation "/Game/Particles/P_Explosion.P_Explosion" (Transformation|GetActorLocation _asmegasphere_c)))))

(event EventTick
  (params (DeltaSeconds :type Float%20%28single-precision%29))
  (Utilities|FlowControl|Sequence
    (:then_0
      ;[1 1 1] Stopwatch timer
      (Utilities|FlowControl|Delay 0.01)
      (Variables|Default|SetSeconds (+ (Variables|Default|GetSeconds) 0.01)))
    (:then_1
      (Utilities|FlowControl|Delay 0.05)
      (Variables|Default|SetP_Points (- (Variables|Default|GetP_Points) 5)))))

(event EventBeginPlay
  ;[1 1 1] Init HUD
  (Audio|PlaySoundatLocation "/Game/Audio/196889__ionicsmusic__race-robot-start.196889__ionicsmusic__race-robot-start" "0, 0, 0")
  (bind _returnvalue (UserInterface|CreateWidget "/Game/Blueprints/PlayerHUD.PlayerHUD_C"))
  (Variables|Default|SetGameHUDWidget _returnvalue)
  (UserInterface|Viewport|AddtoViewport (Variables|Default|GetGameHUDWidget)))

(event Input|ActionEvents|InputActionCollect)

(event Input|KeyboardEvents|SpaceBar
  (:Pressed
    (Variables|Default|SetP_Jumps (+ (Variables|Default|GetP_Jumps) 1))
    (Variables|Default|SetP_Points (- (Variables|Default|GetP_Points) 250))))

(fn ConstructionScript)