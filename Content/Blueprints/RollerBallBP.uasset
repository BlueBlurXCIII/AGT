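; RollerBallBP is a Blueprint, named for a roller ball, that runs a stopwatch and puts the player HUD on screen.
; BeginPlay creates and stores the PlayerHUD widget, while Tick accumulates delta time into Seconds.
; An unconnected sequence holds tiered pickup scoring that adds to PPoints with a sound, but it never runs and casts self rather than an overlapped actor.
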(event EventTick
  (params (DeltaSeconds :type Float%20%28single-precision%29))
  ;[1 1 1] Stopwatch timer
  (Variables|Default|SetSeconds (+ DeltaSeconds (Variables|Default|GetSeconds))))

(event EventBeginPlay
  ;[1 1 1] Init HUD
  (bind _returnvalue (UserInterface|CreateWidget "/Game/Blueprints/PlayerHUD.PlayerHUD_C"))
  (Variables|Default|SetGameHUDWidget _returnvalue)
  (UserInterface|Viewport|AddtoViewport (Variables|Default|GetGameHUDWidget)))

(fn ConstructionScript)